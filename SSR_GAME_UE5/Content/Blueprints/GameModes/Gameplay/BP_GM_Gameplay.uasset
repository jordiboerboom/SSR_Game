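; Gameplay GameMode that gives each joining player a distinct color and applies it to their flags.
; On login it assigns the first unused entry from AvailableColors to the BP_PC_Gameplay controller, and on logout it frees that color.
; Both events then notify the GameState of the connection change and recolor every Plaatsvlag_Actor from its owning controller's assigned color.
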(event `self.ReceiveBeginPlay`
  (`parent.ReceiveBeginPlay`))

(event `self.K2_PostLogin`
  (params (NewPlayer :type "PlayerController Object Reference"))
  (bind _asbp_pc_gameplay (cast `/Game/Blueprints/GameModes/Gameplay/BP_PC_Gameplay` NewPlayer))
  (`self.Assign Player Color` _asbp_pc_gameplay)
  (message `/Game/Blueprints/Interfaces/BPI_Gamestate.NotifyPlayerConnection` (`GameplayStatics.GetGameState`) :!label _label)
  (`self.Refresh Flag Colors`))

(event `self.K2_OnLogout`
  (params (ExitingController :type "Controller Object Reference"))
  (bind _asbp_pc_gameplay (cast `/Game/Blueprints/GameModes/Gameplay/BP_PC_Gameplay` ExitingController))
  (`self.Free Player Color` _asbp_pc_gameplay)
  (goto _label))

(fn `Assign Player Color`
  (params (`Player Controller` :type "/Game/Blueprints/GameModes/Gameplay/BP_PC_Gameplay Object Reference"))
  (for _array_element (`self.Available Colors`)
    (if (not (`KismetArrayLibrary.Array_Contains` (`self.Assigned Colors`) _array_element))
      (break)))
  (bind _output_get (set `/Game/Blueprints/GameModes/Gameplay/BP_PC_Gameplay.AssignedColor` _array_element `Player Controller`))
  (`KismetArrayLibrary.Array_Add` (`self.Assigned Colors`) _output_get))

(fn `Free Player Color`
  (params (`Player Controller` :type "/Game/Blueprints/GameModes/Gameplay/BP_PC_Gameplay Object Reference"))
  (`KismetArrayLibrary.Array_RemoveItem` (`self.Assigned Colors`) (`/Game/Blueprints/GameModes/Gameplay/BP_PC_Gameplay.AssignedColor` `Player Controller`)))

(fn `Refresh Flag Colors`
  (bind _outactors (`GameplayStatics.GetAllActorsOfClass` "/Game/Meubilair/GameObjects/Plaatsvlag_Actor.Plaatsvlag_Actor_C"))
  (for _array_element _outactors
    (bind _asbp_pc_gameplay (cast `/Game/Blueprints/GameModes/Gameplay/BP_PC_Gameplay` (`self.GetOwner` _array_element)))
    (`/Game/Meubilair/GameObjects/Plaatsvlag_Actor.SetFlagColor` _array_element (`/Game/Blueprints/GameModes/Gameplay/BP_PC_Gameplay.AssignedColor` _asbp_pc_gameplay))))

(fn `UserConstructionScript`
  (`parent.UserConstructionScript`))