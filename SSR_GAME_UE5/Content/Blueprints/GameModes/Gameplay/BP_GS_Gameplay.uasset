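; Gameplay game state that runs a replicated pre-match countdown once enough players have connected.
; NotifyPlayerConnection compares the player-state count to MinimumPlayers and starts the countdown once through a DoOnce.
; OnRep_Countdown refreshes every Start_Countdown widget, then on the authority re-triggers the one-second delayed decrement, so the RepNotify itself drives the timer loop.
; At zero the server only prints that the match started.
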(event `/Game/Blueprints/Interfaces/BPI_Gamestate.NotifyPlayerConnection`
  (bind _output_get (set `self.CurrentPlayers` (`GameplayStatics.GetNumPlayerStates`)))
  (if (>= _output_get (`self.MinimumPlayers`))
    (`/Engine/EditorBlueprintResources/StandardMacros.DoOnce` false
      (:`Completed`
        (set `self.Countdown` 30)))))

(event `Match Countdown`
  (`KismetSystemLibrary.Delay` 1.0)
  (set `self.Countdown` (- (`self.Countdown`) 1)))

(fn `OnRep_Countdown`
  (`self.UpdateCountdownWidget`)
  (`/Engine/EditorBlueprintResources/ActorMacros.Switch Has Authority`
    (:`Authority`
      (if (== (`self.Countdown`) 30)
        (`self.Match Countdown`)
        (elif (== (`self.Countdown`) 0)
          (`KismetSystemLibrary.PrintString` "MATCH STARTED")
          (else
            (`self.Match Countdown`)))))))

(fn `UpdateCountdownWidget`
  (bind _foundwidgets (`WidgetBlueprintLibrary.GetAllWidgetsOfClass` "/Game/UI/Start_Countdown.Start_Countdown_C" false))
  (for _array_element _foundwidgets
    (`/Game/UI/Start_Countdown.Update Widget` _array_element (`self.Countdown`))))

(fn `UserConstructionScript`
  (`parent.UserConstructionScript`))