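; BP_PC_Core is a player controller that starts in game-only input and toggles the pause menu on the Pause action.
; The first press creates the Pause_Menu widget and adds it to the viewport; later presses switch the cached widget between Visible and Collapsed.
; Showing the menu enables the cursor with Game and UI input, hiding it restores game-only input, and the game itself is never paused here.
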(event `self.ReceiveBeginPlay`
  (`WidgetBlueprintLibrary.SetInputMode_GameOnly` self))

(event `InputAction|Pause`
  (params (Key :type "Key Structure"))
  (bind _wb_gamemenu (`self.WB_GameMenu`))
  (:`Pressed`
    (`WidgetBlueprintLibrary.SetInputMode_UIOnlyEx` self (`self.WB_GameMenu`))
    (`self.WB_GameMenu`
      (:`then`
        (if (`Widget.IsVisible` (`self.WB_GameMenu`))
          (`Widget.SetVisibility` _wb_gamemenu "Collapsed")
          (set `self.bShowMouseCursor` false)
          (`WidgetBlueprintLibrary.SetInputMode_GameOnly` self)
          (else
            (`Widget.SetVisibility` _wb_gamemenu "Visible")
            (set `self.bShowMouseCursor` true :!label _label)
            (`WidgetBlueprintLibrary.SetInputMode_GameAndUIEx` self (`self.WB_GameMenu`)))))
      (:`else`
        (bind _returnvalue (`|CreateWidget` "/Game/UI/Pause_Menu.Pause_Menu_C" self))
        (bind _output_get (set `self.WB_GameMenu` _returnvalue))
        (`UserWidget.AddToViewport` _output_get 1)
        (goto _label)))))

(fn `UserConstructionScript`)